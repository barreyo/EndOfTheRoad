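; BP_TV is a television prop that switches between a noise state and playback of a Big Buck Bunny video.
; Construction creates a dynamic instance of M_TV on the mesh and starts in the stopped state with TV noise audio.
; Start and stop events set the material's VideoOn parameter and swap sounds, with start also rewinding playback.
; ToggleOnOff sets TvOn on the material, but the nodes flipping its variable are disconnected.
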(event Custom|ToggleOnOff
  (Rendering|Material|SetScalarParameterValue (Variables|Default|GetMaterialTVDisplay) "TvOn" (* (Math|Conversions|ToInteger(Boolean) (not (Variables|Default|GetTvOn))) 1.0) :!class /Script/Engine.MaterialInstanceDynamic))

(event Custom|StartVideo
  (bind _newvar (Variables|Default|GetNewVar))
  (Rendering|Material|SetScalarParameterValue (Variables|Default|GetMaterialTVDisplay) "VideoOn" 1.0 :!class /Script/Engine.MaterialInstanceDynamic)
  (Audio|Components|Audio|SetSound "/Game/Assets/Video/big_buck_bunny_480p_surround-fix_Wav.big_buck_bunny_480p_surround-fix_Wav")
  (Audio|Components|Audio|Play (Variables|Default|GetAudioPlayer) 0.0)
  (Class|MediaPlayer|Rewind _newvar)
  (Media|MediaPlayer|Play _newvar :!class /Script/MediaAssets.MediaPlayer))

(event Custom|StopVideo
  (Rendering|Material|SetScalarParameterValue (Variables|Default|GetMaterialTVDisplay) "VideoOn" 0.0 :!class /Script/Engine.MaterialInstanceDynamic)
  (Audio|Components|Audio|SetSound "/Game/Assets/Audio/SoundEffects/tv-noise_Cue.tv-noise_Cue")
  (Audio|Components|Audio|Play 0.0))

(fn ConstructionScript
  (bind _returnvalue (Rendering|Material|CreateDynamicMaterialInstance 1 "/Game/Materials/M_TV.M_TV" :!class /Script/Engine.PrimitiveComponent))
  (Variables|Default|SetMaterialTVDisplay _returnvalue)
  (CallFunction|StopVideo))