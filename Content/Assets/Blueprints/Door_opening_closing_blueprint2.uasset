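; Interactive door that the player opens and closes with E while overlapping it, with a locked state.
; Overlap toggles input; E plays or reverses the opening timeline when unlocked, or restarts a locked timeline otherwise.
; Both timelines share one rotation lerp, selecting alpha by lock state, while matching sounds play and fade out after opening finishes.
; The construction script applies configurable meshes, derives play rate from opening time and sets the default sound.
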(event Custom|DoorLocked
  ;[1 1 1] Opening/closing animation
  (bind _interpolationalpha (Timeline|Door_locked_animation PlayFromStart)
    (:Update
      (Transformation|SetRelativeRotation (Variables|Default|GetDoor) (Math|Rotator|Lerp(Rotator) (Variables|Default|GetDoor%20start) (Variables|Default|GetDoor%20end) (Math|Float|SelectFloat (stale Custom|DoorOpen _interpolationalpha) _interpolationalpha (Variables|Default|GetDoor%20unlocked))) false))))

(event Custom|DoorOpen
  ;[1 1 1] Opening/closing animation
  (bind _interpolationalpha (Timeline|Door_opening_animation Play)
    (:Update
      (Transformation|SetRelativeRotation (Variables|Default|GetDoor) (Math|Rotator|Lerp(Rotator) (Variables|Default|GetDoor%20start) (Variables|Default|GetDoor%20end) (Math|Float|SelectFloat _interpolationalpha (stale Custom|DoorLocked _interpolationalpha) (Variables|Default|GetDoor%20unlocked))) false))
    (:Finished
      (Audio|Components|Audio|FadeOut 0.3 0.0 :!class /Script/Engine.AudioComponent))))

(event Custom|DoorClose
  ;[1 1 1] Opening/closing animation
  (bind _interpolationalpha (Timeline|Door_opening_animation Reverse)
    (:Update
      (Transformation|SetRelativeRotation (Variables|Default|GetDoor) (Math|Rotator|Lerp(Rotator) (Variables|Default|GetDoor%20start) (Variables|Default|GetDoor%20end) (Math|Float|SelectFloat _interpolationalpha (stale Custom|DoorLocked _interpolationalpha) (Variables|Default|GetDoor%20unlocked))) false))
    (:Finished
      (Audio|Components|Audio|FadeOut 0.3 0.0 :!class /Script/Engine.AudioComponent))))

(event EventActorBeginOverlap
  (params (OtherActor :type Actor%20Object%20Reference))
  ;[1 1 1] Setup input enabling/disabling
  (Input|EnableInput (Game|GetPlayerController 0)))

(event EventActorEndOverlap
  (params (OtherActor :type Actor%20Object%20Reference))
  ;[1 1 1] Setup input enabling/disabling
  (Input|DisableInput (Game|GetPlayerController 0)))

(event Input|KeyboardEvents|E
  (bind _audioplayer (Variables|Default|GetAudioPlayer))
  ;[1 1 1] Door opening logic
  (:Pressed
    (if (Variables|Default|GetDoor%20unlocked)
      (if (Variables|Default|GetDoor%20open)
        (CallFunction|DoorClose)
        (else
          (CallFunction|DoorOpen)))
      (Variables|Default|SetDoor%20open (not (Variables|Default|GetDoor%20open)))
      ;[1 1 1] Enable audio
      (Audio|Components|Audio|SetSound _audioplayer (Variables|Default|GetUnlocked%20Sound%20Asset))
      (else
        (CallFunction|DoorLocked)
        (Audio|Components|Audio|SetSound _audioplayer (Variables|Default|GetLocked%20Sound%20Asset))))
    (Audio|Components|Audio|Stop _audioplayer)
    (Audio|Components|Audio|Play _audioplayer 0.0)))

(fn ConstructionScript
  ;[1 1 1] Set door and frame meshes
  (Components|StaticMesh|SetStaticMesh (Variables|Default|GetFrame%20model))
  (Components|StaticMesh|SetStaticMesh (Variables|Default|GetDoor%20model))
  ;[1 1 1] Set opening/closing speed
  (Components|Timeline|SetPlayRate (/ 1.0 (Variables|Default|GetOpening%20time)))
  (Variables|/Script/Engine.AudioComponent|SetSound (Variables|Default|GetAudioPlayer) (Variables|Default|GetUnlocked%20Sound%20Asset)))