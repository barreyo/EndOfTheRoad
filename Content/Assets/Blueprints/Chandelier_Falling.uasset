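; Chandelier actor that drops when something overlaps its trigger box.
; On overlap, it turns on physics simulation for the chandelier mesh and hides its twelve point lights, with no filter on the overlapping actor.
; The construction script applies the light color and intensity variables to all the lights and moves the trigger box to a configurable relative position, so each placed instance can be tuned.
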(event OnComponentBeginOverlap(TriggerBox)
  (params (OtherActor :type Actor%20Object%20Reference) (OtherComp :type Primitive%20Component%20Object%20Reference) (OtherBodyIndex :type Integer) (bFromSweep :type Boolean) (SweepResult :type Hit%20Result%20Structure%20%28by%20ref%29))
  (Physics|SetSimulatePhysics (Variables|Default|GetChandelier) true)
  (Rendering|SetVisibility (Variables|Default|GetPointLight1) false false))

(fn ConstructionScript
  (Rendering|Components|Light|SetLightColor (Variables|Default|GetPointLight2) (Variables|Default|GetLightColor))
  (Transformation|SetRelativeLocation (Variables|Default|GetTriggerBox) (Variables|Default|GetTriggerPosition) false)
  (Rendering|Components|Light|SetIntensity (Variables|Default|GetPointLight1) (Variables|Default|GetIntensity)))