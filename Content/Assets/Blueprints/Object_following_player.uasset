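; Blueprint object that slides its mesh along a plane to follow the player character.
; Start and stop events toggle following, and each tick moves the mesh only while following and enabled.
; The player location is projected onto a plane through the mesh using a configurable normal.
; A FollowZ flag, used as an integer multiplier, chooses between the projected height and the mesh's current height.
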(event Custom|StartFollowingPlayer
  ;[1 1 1] Enable and disable following
  (Variables|Default|SetFollowing (Class|KismetSystemLibrary|MakeLiteralBool true)))

(event Custom|StopFollowingPlayer
  ;[1 1 1] Enable and disable following
  (Variables|Default|SetFollowing (Class|KismetSystemLibrary|MakeLiteralBool false)))

(event EventTick
  (params (DeltaSeconds :type Float%20%28single-precision%29))
  (bind _returnvalue (Game|GetPlayerCharacter 0))
  (bind _follow_z (Variables|Default|GetFollow%20Z))
  (bind _mesh (Variables|Default|GetMesh))
  (bind _plane_normal (Variables|Default|GetPlane%20normal))
  (bind _returnvalue_2 (Math|Vector|Normalize _plane_normal))
  (bind _returnvalue_3 (Transformation|GetActorLocation _returnvalue))
  (bind _returnvalue_4 (Transformation|GetWorldLocation _mesh))
  (bind _returnvalue_5 (Class|KismetMathLibrary|ProjectPointontoPlane _returnvalue_3 _returnvalue_4 _returnvalue_2))
  (bind (_x _y _z) (Math|Vector|BreakVector _returnvalue_5))
  ;[1 1 1] Follow player
  (if (and (Variables|Default|GetFollowing) (Variables|Default|GetEnabled))
    (Transformation|SetWorldLocation (Variables|Default|GetMesh) (Math|Vector|MakeVector _x _y (+ (* (Math|Conversions|ToInteger(Boolean) _follow_z) _z) (* (Math|Conversions|ToInteger(Boolean) (not _follow_z)) (.Z (Math|Vector|BreakVector _returnvalue_4))))) false)))

(fn ConstructionScript)