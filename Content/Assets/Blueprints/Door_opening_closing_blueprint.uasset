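; An interactive door that the player opens and closes with the E key, or rattles when it is locked.
; Actor overlap enables and disables input from player controller 0, so E works only in range.
; If unlocked, E toggles a timeline forward or in reverse; otherwise it restarts a locked timeline.
; Both timelines share one rotation lerp between start and end, selecting their alpha by the unlocked flag.
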(event Custom|DoorLocked
  ;[1 1 1] Opening/closing animation
  (bind _interpolationalpha (Timeline|Door_locked_animation PlayFromStart)
    (:Update
      (Transformation|SetRelativeRotation (Variables|Default|GetDoor) (Math|Rotator|Lerp(Rotator) (Variables|Default|GetDoorStart) (Variables|Default|GetDoorEnd) (Math|Float|SelectFloat (stale Custom|DoorOpen _interpolationalpha) _interpolationalpha (Variables|Default|GetDoorUnlocked))) false))))

(event Custom|DoorOpen
  ;[1 1 1] Opening/closing animation
  (bind _interpolationalpha (Timeline|Door_opening_animation Play)
    (:Update
      (Transformation|SetRelativeRotation (Variables|Default|GetDoor) (Math|Rotator|Lerp(Rotator) (Variables|Default|GetDoorStart) (Variables|Default|GetDoorEnd) (Math|Float|SelectFloat _interpolationalpha (stale Custom|DoorLocked _interpolationalpha) (Variables|Default|GetDoorUnlocked))) false))))

(event Custom|DoorClose
  ;[1 1 1] Opening/closing animation
  (bind _interpolationalpha (Timeline|Door_opening_animation Reverse)
    (:Update
      (Transformation|SetRelativeRotation (Variables|Default|GetDoor) (Math|Rotator|Lerp(Rotator) (Variables|Default|GetDoorStart) (Variables|Default|GetDoorEnd) (Math|Float|SelectFloat _interpolationalpha (stale Custom|DoorLocked _interpolationalpha) (Variables|Default|GetDoorUnlocked))) false))))

(event EventActorBeginOverlap
  (params (OtherActor :type Actor%20Object%20Reference))
  ;[1 1 1] Setup input enabling/disabling
  (Input|EnableInput (Game|GetPlayerController 0)))

(event EventActorEndOverlap
  (params (OtherActor :type Actor%20Object%20Reference))
  ;[1 1 1] Setup input enabling/disabling
  (Input|DisableInput (Game|GetPlayerController 0)))

(event Input|KeyboardEvents|E
  ;[1 1 1] Door opening logic
  (:Pressed
    (if (Variables|Default|GetDoorUnlocked)
      (if (Variables|Default|GetDoorOpened)
        (CallFunction|DoorClose)
        (else
          (CallFunction|DoorOpen)))
      (Variables|Default|SetDoorOpened (not (Variables|Default|GetDoorOpened)))
      (else
        (CallFunction|DoorLocked)))))

(fn ConstructionScript)