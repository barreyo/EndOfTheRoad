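; Bedside table Blueprint with a drawer that toggles open and closed through the ToggleDrawer event.
; The IsOut flag selects between easing the Drawer component to the Position offset and returning it with zero rotation and no explicit target location.
; Both directions use MoveComponentTo over Duration and play the same OpenDrawer sound.
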(event Custom|Toggle%20Drawer
  (bind _opendrawer (Variables|Default|GetopenDrawer))
  (bind _drawer (Variables|Default|Getdrawer))
  (bind _duration (Variables|Default|Getduration))
  ;[1 1 1] Handle the button click, play sound and open drawer
  (if (Variables|Default|GetisOut)
    (Audio|Components|Audio|Play _opendrawer 0.0)
    (Components|MoveComponentTo _drawer "0, 0, 0" "0.000000, 0,0.000000" false true _duration)
    (Variables|Default|SetisOut false)
    (else
      (Audio|Components|Audio|Play _opendrawer 0.0)
      (Components|MoveComponentTo _drawer (Variables|Default|Getposition) "0, 0, 0" false true _duration)
      (Variables|Default|SetisOut true))))

(fn ConstructionScript)