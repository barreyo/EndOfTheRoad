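; Ceiling light Blueprint with a switchable on/off state, configurable intensity and color, and a glowing glass material.
; The construction script creates the dynamic material, picks static or dynamic point light via UseStatic, and calls ToggleLight twice to refresh without changing state.
; ToggleLight flips LightOn, updates dynamic light visibility, color and material glow, then calls Play.
; The static light's visibility update in the event graph is disconnected.
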(event Custom|ToggleLight
  (bind _lightcolor (Variables|Default|GetLightColor))
  (bind _material (Variables|Default|GetMaterial))
  (Variables|Default|SetLightOn (not (Variables|Default|GetLightOn)))
  (Rendering|SetVisibility (Variables|Default|GetPointLightDynamic) (and (Variables|Default|GetLightOn) (not (Variables|Default|GetUseStatic))) false)
  (Rendering|Material|SetScalarParameterValue _material "LightIntensity" (Math|Float|SelectFloat (/ (Variables|Default|GetIntensity) 6e+01) 0.0 (Variables|Default|GetLightOn)) :!class /Script/Engine.MaterialInstanceDynamic)
  (Rendering|Material|SetVectorParameterValue _material "LightColor" _lightcolor :!class /Script/Engine.MaterialInstanceDynamic)
  (Rendering|Components|Light|SetLightColor (Variables|Default|GetPointLightDynamic) _lightcolor)
  (Audio|Components|Audio|Play 0.0))

(fn ConstructionScript
  (bind _lightcolor (Variables|Default|GetLightColor))
  (bind _intensity (Variables|Default|GetIntensity))
  (bind _returnvalue (Rendering|Material|CreateDynamicMaterialInstance 0 "/Game/StarterContent/Materials/M_Glass_Glowing.M_Glass_Glowing" :!class /Script/Engine.PrimitiveComponent))
  (Variables|Default|SetMaterial _returnvalue)
  (Rendering|SetVisibility (and (Variables|Default|GetLightOn) (not (Variables|Default|GetUseStatic))) false)
  (Rendering|SetVisibility (and (Variables|Default|GetLightOn) (Variables|Default|GetUseStatic)) false)
  (CallFunction|ToggleLight)
  (CallFunction|ToggleLight)
  (Rendering|Components|Light|SetIntensity _intensity)
  (Rendering|Components|Light|SetIntensity _intensity)
  (Rendering|Material|SetVectorParameterValue (Variables|Default|GetMaterial) "LightColor" _lightcolor :!class /Script/Engine.MaterialInstanceDynamic)
  (Rendering|Components|Light|SetLightColor (Variables|Default|GetPointLightDynamic) _lightcolor))