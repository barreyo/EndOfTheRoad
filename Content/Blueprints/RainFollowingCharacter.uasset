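; Rain effect actor that keeps its rain over the player character.
; Each Tick copies the player's X and Y into a world-location update while taking height from the RainSystem component.
; TurnOn and TurnOff events activate or deactivate the RainSystem and Impact effects together, printing the emitter state.
; The construction script calls TurnOffEvent.
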(event Custom|TurnOn_Event
  (Components|Activation|Activate (Variables|Default|Getimpact) false)
  (Components|Activation|Activate (Variables|Default|GetRainSystem) false)
  (Development|PrintString "Emitter On"))

(event Custom|TurnOff_Event
  (Components|Activation|Deactivate (Variables|Default|Getimpact))
  (Components|Activation|Deactivate (Variables|Default|GetRainSystem))
  (Development|PrintString "Emitter Off"))

(event EventTick
  (params (DeltaSeconds :type Float%20%28single-precision%29))
  (bind _returnvalue (Game|GetPlayerCharacter 0))
  (bind _returnvalue_2 (Transformation|GetWorldLocation _returnvalue))
  (bind (_x _y) (Math|Vector|BreakVector _returnvalue_2))
  (Transformation|SetWorldLocation (Math|Vector|MakeVector _x _y (.Z (Math|Vector|BreakVector (Transformation|GetWorldLocation (Variables|Default|GetRainSystem))))) false))

(fn ConstructionScript
  (CallFunction|TurnOffEvent))