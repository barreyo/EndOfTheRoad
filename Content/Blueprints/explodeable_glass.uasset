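; Glass Blueprint that can be made to shatter outward on demand, with the explosion behavior switchable on and off.
; EnableGlassExplosion and DisableGlassExplosion set a ShouldExplode flag that gates the ExplodeGlass event.
; When allowed, ExplodeGlass applies small-radius damage at the center of mass, with impulse strength taken from the ExplosionStrength variable.
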(event Custom|Explode%20Glass
  ;[1 1 1] Make things go boom
  (if (Variables|Default|GetShould%20Explode)
    (bind _returnvalue (Physics|GetCenterOfMass "None"))
    (Class|DestructibleComponent|ApplyRadiusDamage 1e+01 _returnvalue 1e+01 (Variables|Default|GetExplosion%20strength) false)))

(event Custom|EnableGlassExplosion
  ;[1 1 1] Enable and disable explosions
  (Variables|Default|SetShould%20Explode (Class|KismetSystemLibrary|MakeLiteralBool true)))

(event Custom|DisableGlassExplosion
  ;[1 1 1] Enable and disable explosions
  (Variables|Default|SetShould%20Explode (Class|KismetSystemLibrary|MakeLiteralBool false)))

(fn ConstructionScript)