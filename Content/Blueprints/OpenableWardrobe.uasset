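; Wardrobe Blueprint with two doors that swing open independently through the OpenLeft and OpenRight events.
; Each event plays its own timeline to interpolate that door's relative yaw to OpeningAngle, with the right door holding a 180-degree roll as a flipped counterpart.
; The construction script derives timeline play rates from DoorsOpeningTime and applies configurable materials to the body, doors and doorknobs.
; No closing logic is present.
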(event Custom|OpenRight
  (bind _rotation (Timeline|RightDoorOpen Play)
    (:Update
      (Transformation|SetRelativeRotation (Math|Rotator|Lerp(Rotator) "0, 0,180.000000" (Class|KismetMathLibrary|MakeRot 0.0 (Variables|Default|GetOpeningAngle) 1.8e+02) _rotation) false))))

(event Custom|OpenLeft
  (bind _rotation (Timeline|LeftDoorOpen Play)
    (:Update
      (Transformation|SetRelativeRotation (Math|Rotator|Lerp(Rotator) "0, 0, 0" (Class|KismetMathLibrary|MakeRot 0.0 (Variables|Default|GetOpeningAngle) 0.0) _rotation) false))))

(fn ConstructionScript
  (bind _doorsopeningtime (Variables|Default|GetDoorsOpeningTime))
  (bind _doorsmaterial (Variables|Default|GetDoorsMaterial))
  (bind _returnvalue (/ 1.0 _doorsopeningtime))
  (Components|Timeline|SetPlayRate _returnvalue)
  (Components|Timeline|SetPlayRate _returnvalue)
  (Rendering|Material|SetMaterial 0 (Variables|Default|GetWardrobeMaterial))
  (Rendering|Material|SetMaterial 1 _doorsmaterial)
  (Rendering|Material|SetMaterial 1 _doorsmaterial)
  (Rendering|Material|SetMaterial 0 (Variables|Default|GetDoorknobMaterials))
  (Rendering|Material|SetMaterial 0 0))