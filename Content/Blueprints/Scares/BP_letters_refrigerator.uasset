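; Refrigerator letters scare: letter components U, R, N, X and T slide and tilt into new positions when the movement event is played.
; PlayLetterMovement_Event runs once through a DoOnce, starting LetterU on an eased MoveComponentTo to an offset from its current location and printing a debug string.
; Staggered timers fire per-letter events that ease the other four toward stored end-location variables, each with its own rotation and duration.
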(event Custom|PlayLetterMovement_Event
  (bind _letteru (Variables|Default|GetLetterU))
  (bind _relativelocation (Variables|/Script/Engine.SceneComponent|GetRelativeLocation _letteru))
  (bind (_x _y _z) (Math|Vector|BreakVector _relativelocation))
  (Utilities|FlowControl|DoOnce false
    (:Completed
      (Utilities|Time|SetTimerbyEvent (delegate Custom|MoveLetterR_Event) 0.5)
      (Utilities|Time|SetTimerbyEvent (delegate Custom|MoveLetterN_Event) 0.8)
      (Utilities|Time|SetTimerbyEvent (delegate Custom|MoveLetterX_Event) 1.0)
      (Utilities|Time|SetTimerbyEvent (delegate Custom|MoveLetterT_Event) 1.1)
      (Components|MoveComponentTo _letteru (Math|Vector|MakeVector _x (+ _y -1.0) (+ _z 34.0)) "0, 0,-20.000000" true true 1.2)
      (Development|PrintString "played yo"))))

(event Custom|MoveLetterR_Event
  (Components|MoveComponentTo (Variables|Default|GetLetterR) (Variables|Default|GetEndLocationR) "0, 0,2.000000" true true 1.0))

(event Custom|MoveLetterN_Event
  (Components|MoveComponentTo (Variables|Default|GetLetterN) (Variables|Default|GetEndLocationN) "0, 0,6.000000" true true 0.8))

(event Custom|MoveLetterX_Event
  (Components|MoveComponentTo (Variables|Default|GetLetterX) (Variables|Default|GetEndLocationX) "0, 0,3.000000" true true 0.7))

(event Custom|MoveLetterT_Event
  (Components|MoveComponentTo (Variables|Default|GetLetterT) (Variables|Default|GetEndLocationT) "0, 0,10.000000" true true 0.5))

(fn ConstructionScript)