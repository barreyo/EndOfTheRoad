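; BP_AmbientSoundController switches ambient audio between inside and outside states.
; Two custom events, TurnOnInsideSound and TurnOnOutsideSound, each check and update an Inside flag so repeated calls do nothing.
; Each switch calls FadeOut and then FadeIn, with a gradual fade-out when going inside and instant fades when going outside.
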(event Custom|TurnOnOutsideSound
  (if (Variables|Default|Getinside)
    (Audio|Components|Audio|FadeOut 0.0 0.0 :!class /Script/Engine.AudioComponent)
    (Audio|Components|Audio|FadeIn 0.0 1.0 0.0 :!class /Script/Engine.AudioComponent)
    (Variables|Default|Setinside false)))

(event Custom|TurnOnInsideSound
  (if (not (Variables|Default|Getinside))
    (Audio|Components|Audio|FadeOut 3.0 0.0 :!class /Script/Engine.AudioComponent)
    (Audio|Components|Audio|FadeIn 0.0 1.0 0.0 :!class /Script/Engine.AudioComponent)
    (Variables|Default|Setinside true)))

(fn ConstructionScript)