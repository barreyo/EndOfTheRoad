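; DangerousWardrobe is an interactive horror prop: a wardrobe whose doors open to release a falling axe.
; Overlapping the trigger box enables player 0's input so E can start it; leaving disables that input.
; The left-door timeline's updates drive the right-door timeline, whose completion plays a horror sound and starts the axe-fall timeline.
; One second after the fall finishes, two components are destroyed.
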(event OnComponentBeginOverlap(TriggerBox)
  (params (OtherActor :type Actor%20Object%20Reference) (OtherComp :type Primitive%20Component%20Object%20Reference) (OtherBodyIndex :type Integer) (bFromSweep :type Boolean) (SweepResult :type Hit%20Result%20Structure%20%28by%20ref%29))
  ;[1 1 1] Enable/Disable input
  (Input|EnableInput (Game|GetPlayerController 0)))

(event OnComponentEndOverlap(TriggerBox)
  (params (OtherActor :type Actor%20Object%20Reference) (OtherComp :type Primitive%20Component%20Object%20Reference) (OtherBodyIndex :type Integer))
  ;[1 1 1] Enable/Disable input
  (Input|DisableInput (Game|GetPlayerController 0)))

(event Input|KeyboardEvents|E
  (:Pressed
    ;[1 1 1] Open doors logic
    (bind _doorrotation (Timeline|OpenLeft Play)
      (:Update
        (Transformation|SetRelativeRotation (Class|KismetMathLibrary|MakeRot 0.0 _doorrotation 0.0) false)
        (bind _doorrotation_2 (Timeline|OpenRight Play)
          (:Update
            (Transformation|SetRelativeRotation (Class|KismetMathLibrary|MakeRot 0.0 _doorrotation_2 1.8e+02) false))
          (:Finished
            ;[1 1 1] Play sound
            (Audio|Components|Audio|Play (Variables|Default|GetHorrorSound) 0.0)
            ;[1 1 1] Make the axe fall
            (bind _fall (Timeline|FallingAxe Play)
              (:Update
                (Transformation|SetRelativeRotation (Class|KismetMathLibrary|MakeRot _fall 0.0 9e+01) false))
              (:Finished
                ;[1 1 1] Destroy components
                (Utilities|FlowControl|Delay 1.0)
                (Components|DestroyComponent)
                (Components|DestroyComponent)))))))))

(fn ConstructionScript)