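; Bookshelf prop that topples once when TriggerFall is called, playing its Hit effect, likely a sound, as it starts.
; TriggerFall enables physics and applies a force at a set location on the Shelf to tip it over.
; Impacts above a minimum impulse replay Hit until, after a short delay, the shelf is flagged as on the floor and physics is switched off.
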(event Custom|Trigger%20Fall
  (if (not (Variables|Default|GetTriggered))
    (Variables|Default|SetTriggered true)
    (Physics|SetSimulatePhysics true)
    (Class|PrimitiveComponent|AddForceatLocation (Variables|Default|GetShelf) (Variables|Default|GetForce) (Variables|Default|GetLocation%20of%20force) "None")
    (Audio|Components|Audio|Play (Variables|Default|GetHit) 0.0)))

(event EventHit
  (params (MyComp :type Primitive%20Component%20Object%20Reference) (Other :type Actor%20Object%20Reference) (OtherComp :type Primitive%20Component%20Object%20Reference) (bSelfMoved :type Boolean) (HitLocation :type Vector :default "0, 0, 0") (HitNormal :type Vector :default "0, 0, 0") (NormalImpulse :type Vector :default "0, 0, 0") (Hit :type Hit%20Result%20Structure%20%28by%20ref%29))
  (if (and (>= (Math|Vector|VectorLength NormalImpulse) (Variables|Default|GetMinimumImpulse)) (not (Variables|Default|GetOnFloor)))
    (Audio|Components|Audio|Play (Variables|Default|GetHit) 0.0)
    (Utilities|FlowControl|Delay 1.0)
    (Variables|Default|SetOnFloor true)
    (Physics|SetSimulatePhysics false)))

(fn ConstructionScript)